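; BP_milk is a collectible milk pickup that rewards the main character on touch.
; When the SpriteMilk component overlaps main_character, it calls MilkCollect on the character, adds to SweetPoints, resets ShakeProgress to zero and destroys itself.
; Tick spins the actor steadily around its local yaw axis, scaled by delta time.
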(event OnComponentBeginOverlap(spriteMilk)
  (params (OverlappedComponent :type Primitive%20Component%20Object%20Reference) (OtherActor :type Actor%20Object%20Reference) (OtherComp :type Primitive%20Component%20Object%20Reference) (OtherBodyIndex :type Integer) (bFromSweep :type Boolean) (SweepResult :type Hit%20Result%20Structure%20%28by%20ref%29))
  (bind _asmain_character (Utilities|Casting|CastTomain_character OtherActor))
  (Default|MilkCollect _asmain_character)
  (Variables|/Game/main_character.main_character_C|SetSweetPoints _asmain_character (+ (Variables|/Game/main_character.main_character_C|GetSweetPoints _asmain_character) 2))
  (Variables|/Game/main_character.main_character_C|SetShakeProgress _asmain_character 0)
  (Actor|DestroyActor))

(event EventBeginPlay)

(event Collision|EventActorBeginOverlap
  (params (OtherActor :type Actor%20Object%20Reference)))

(event EventTick
  (params (DeltaSeconds :type Float%20%28single-precision%29))
  (Transformation|AddActorLocalRotation (Math|Rotator|MakeRotator 0.0 0.0 (* DeltaSeconds 1.8e+02)) false false))

(fn ConstructionScript)